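; BP_HotPotato is a component that reports hot-potato holding time to a character's player controller.
; Init casts the given character's controller to PC_Gameplay, then starts a looping timer at TimeBetweenTicks.
; Each tick passes that fixed interval to SetTotalTime on the controller, and GetTimeElapsed returns the same interval rather than a running total.
; Detatch clears the counting flag and destroys the component.
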(event `Init`
  (params (CharToApply :type "Pawn Object Reference"))
  (set `self.IsCounting` true)
  (bind _aspc_gameplay (cast `/Game/S020301L/Blueprints/PlayerControllers/PC_Gameplay` (`Pawn.GetController` CharToApply)))
  (`KismetSystemLibrary.K2_SetTimerDelegate` (delegate `Increment`) (`self.TimeBetweenTicks`) (`self.IsCounting`)))

(event `Increment`
  (`/Game/S020301L/Blueprints/PlayerControllers/PC_Gameplay.SetTotalTime` (stale `Init` _aspc_gameplay) (`self.TimeBetweenTicks`)))

(event `Detatch`
  (set `self.IsCounting` false)
  (`self.K2_DestroyComponent`))

(fn `GetTimeElapsed`
  (returns (TimeElapsed :type "Float (double-precision)"))
  (return (`self.TimeBetweenTicks`)))