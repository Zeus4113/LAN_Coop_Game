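; Game mode for a local multiplayer HP match in which the player with the lowest total time wins.
; Creates players from game-instance settings, assigns teams with a random pick for Team B, and disables input during a timed pre-game.
; In-game spawns BP_GameManager with the controllers and binds its timer completion.
; Post-game shows each player the winner, then a time-dilation timeline ends in player removal and a return to the main menu.
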(event `self.ReceiveBeginPlay`
  (bind _output_get (set `self.GameInstance` (cast `/Game/S020301L/Blueprints/BP_GameInstance` (`GameplayStatics.GetGameInstance`) :!pure true)))
  (bind _gamesettings (`/Game/S020301L/Blueprints/BP_GameInstance.GetGameSettings` _output_get))
  (`self.Set Up Controllers` (`.Players_6_7B2077B54F1A3293A9B042B52C5B4AB6` (break `/Game/S020301L/Blueprints/Data/BPS_GameSettings` _gamesettings)))
  (`self.SwitchGameStates` "NewEnumerator0")
  (`KismetSystemLibrary.K2_SetTimerDelegate` (delegate `Pre-Game Delay`) 3.0))

(event `Pre-Game Delay`
  (`self.SwitchGameStates` "NewEnumerator1"))

(event `DilateTime`
  (bind (_direction _newtrack_0) (`Timeline|DilationTimeline`)
    (:`Update`
      (`GameplayStatics.SetGlobalTimeDilation` _newtrack_0))
    (:`Finished`
      (`GameplayStatics.SetGlobalTimeDilation` 1.0)
      (`/Game/S020301L/Blueprints/Data/BPL_Gameplay.Remove Players`)
      (bind _returnvalue (`GameplayStatics.CreatePlayer` 0))
      (message `/Game/S020301L/Blueprints/Interfaces/BPI_Initialisable.Init` _returnvalue)
      (`GameplayStatics.OpenLevel` "MainMenu_Map"))))

(event `self.K2_PostLogin`
  (params (NewPlayer :type "PlayerController Object Reference"))
  ;[1 0.3124 0.3224] Login / Logout Events
  (bind _aspc_gameplay (cast `/Game/S020301L/Blueprints/PlayerControllers/PC_Gameplay` NewPlayer))
  (`KismetArrayLibrary.Array_Add` (`self.Player Controllers`) _aspc_gameplay))

(event `self.K2_OnLogout`
  (params (ExitingController :type "Controller Object Reference"))
  ;[1 0.3124 0.3224] Login / Logout Events
  (bind _aspc_gameplay (cast `/Game/S020301L/Blueprints/PlayerControllers/PC_Gameplay` ExitingController))
  (`KismetArrayLibrary.Array_RemoveItem` (`self.Player Controllers`) _aspc_gameplay)
  (`KismetArrayLibrary.Array_RemoveItem` (`self.TeamA_Controllers`) _aspc_gameplay)
  (`KismetArrayLibrary.Array_RemoveItem` (`self.TeamB_Controllers`) _aspc_gameplay))

(fn `AddToTeamList`
  (params (PC_Gameplay :type "/Game/S020301L/Blueprints/PlayerControllers/PC_Gameplay Object Reference"))
  (bind _team_id (`/Game/S020301L/Blueprints/Interfaces/BPI_Teams.GetTeam` PC_Gameplay))
  (switch `/Game/S020301L/Blueprints/Data/E_Teams` _team_id
    (:`NewEnumerator1`
      (`KismetArrayLibrary.Array_Add` (`self.TeamA_Controllers`) PC_Gameplay))
    (:`NewEnumerator2`
      (`KismetArrayLibrary.Array_Add` (`self.TeamB_Controllers`) PC_Gameplay))))

(fn `ChoosePlayerStart`
  (params (Player :type "Controller Object Reference"))
  (returns (ReturnValue :type "Actor Object Reference"))
  (return null))

(fn `FindLowestTime`
  (returns (WinningTime :type "Float (double-precision)") (PlayerNum :type Integer))
  (locals (PlayerNumber :type Integer))
  (bind _winningtime (`self.WinningTime`))
  (for _array_element (`self.Player Controllers`)
    (bind _timeaspotato (`/Game/S020301L/Blueprints/PlayerControllers/PC_Gameplay.GetTotalTime` _array_element))
    (`KismetArrayLibrary.Array_Add` (`self.PlayerTimes`) _timeaspotato))
  (for (_array_element_2 _array_index) (`self.PlayerTimes`)
    (if (< _array_element_2 _winningtime)
      (set `self.WinningTime` _array_element_2)
      (set `local.PlayerNumber` _array_index)))
  (return _winningtime (`local.PlayerNumber`)))

(fn `GetGameManager`
  (returns (GameManager :type "/Game/S020301L/Blueprints/BP_GameManager Object Reference"))
  (return (`self.GameManager`)))

(fn `GetTeam`
  (returns (`Team ID` :type "/Game/S020301L/Blueprints/Data/E_Teams Enum"))
  (return "NewEnumerator0"))

(fn `In-Game Setup`
  (bind _returnvalue (`|SpawnActorFromClass` "/Game/S020301L/Blueprints/BP_GameManager.BP_GameManager_C" (`KismetMathLibrary.MakeTransform` (0.0 0.0 0.0)) "Undefined" "OverrideRootScale" null null))
  (bind _output_get (set `self.GameManager` _returnvalue))
  (add `/Game/S020301L/Blueprints/BP_GameManager.TimerComplete` _output_get (`|CreateDelegate` :!event `Post-Game Setup`))
  (`/Game/S020301L/Blueprints/BP_GameManager.Init` _output_get (`self.Player Controllers`)))

(fn `Post-Game Setup`
  (bind _player_controllers (`self.Player Controllers`))
  (bind (_winningtime _playernum) (`self.FindLowestTime`))
  (`self.DilateTime`)
  (for _array_element _player_controllers
    (bind _output (`/Game/S020301L/Blueprints/PlayerControllers/PC_Gameplay.GetAttachedWidget` _array_element))
    (`Widget.RemoveFromParent` _output))
  (for _array_element_2 _player_controllers
    (bind _returnvalue (`|CreateWidget` "/Game/S020301L/UI/UI_PostGame.UI_PostGame_C" _array_element_2))
    (`/Game/S020301L/UI/UI_PostGame.UpdateText` _returnvalue _playernum)
    (`UserWidget.AddToPlayerScreen` _returnvalue 0)))

(fn `Pre-Game Setup`
  (`self.SetTeams`)
  (`self.SetInput` false)
  (return))

(fn `Set Up Controllers`
  (params (`Number of Players` :type Integer))
  (`GameplayStatics.RemovePlayer` (`GameplayStatics.GetPlayerController` 0))
  (for _index (range `Number of Players`)
    (bind _returnvalue (`GameplayStatics.CreatePlayer` _index))
    (message `/Game/S020301L/Blueprints/Interfaces/BPI_Initialisable.Init` _returnvalue)
    (message `/Game/S020301L/Blueprints/Interfaces/BPI_Teams.SetTeam` _returnvalue "NewEnumerator0")))

(fn `SetInput`
  (params (`CanInput?` :type Boolean))
  (for _array_element (`self.Player Controllers`)
    (`/Game/S020301L/Blueprints/PlayerControllers/PC_Gameplay.CanInput` _array_element `CanInput?`)))

(fn `SetTeams`
  (locals (ChaserIndex :type Integer :default 0))
  (bind _player_controllers (`self.Player Controllers`))
  (bind _outitem (`KismetArrayLibrary.Array_Random` _player_controllers))
  (for _array_element _player_controllers
    (message `/Game/S020301L/Blueprints/Interfaces/BPI_Teams.SetTeam` _array_element "NewEnumerator1")
    (`self.AddToTeamList` _array_element))
  (message `/Game/S020301L/Blueprints/Interfaces/BPI_Teams.SetTeam` _outitem "NewEnumerator2")
  (`self.AddToTeamList` _outitem))

(fn `SwitchGameStates`
  (params (NewGameState :type "/Game/S020301L/Blueprints/Data/E_GameState Enum" :default "NewEnumerator0"))
  (switch `/Game/S020301L/Blueprints/Data/E_GameState` NewGameState
    (:`NewEnumerator0`
      (`self.Pre-Game Setup`)
      (`KismetSystemLibrary.PrintString` "Pre-Game Setup"))
    (:`NewEnumerator1`
      (`self.In-Game Setup`)
      (`KismetSystemLibrary.PrintString` "In-Game Setup"))
    (:`NewEnumerator2`
      (`self.Post-Game Setup`)
      (`KismetSystemLibrary.PrintString` "Post-Game Setup"))))

(fn `UserConstructionScript`)