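; Game mode for a local multiplayer lava survival round, despite the KOTH name, run as Pre-Game, In-Game and Post-Game states.
; It creates local players from game instance settings, then spawns their chosen characters at random PlayerStarts with input disabled during a HUD countdown.
; In-Game enables input and starts BP_LavaManager, while CheckIfEnd ends play once all players spectate.
; Post-Game shows win or lose widgets by spectating status and starts a timer.
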(event `self.ReceiveBeginPlay`
  (`KismetSystemLibrary.PrintString` "KOTH Loaded")
  (bind _output_get (set `self.GameInstance` (cast `/Game/S020301L/Blueprints/BP_GameInstance` (`GameplayStatics.GetGameInstance`) :!pure true)))
  (bind _gamesettings (`/Game/S020301L/Blueprints/BP_GameInstance.GetGameSettings` _output_get))
  (`self.Set Up Controllers` (`.Players_6_7B2077B54F1A3293A9B042B52C5B4AB6` (break `/Game/S020301L/Blueprints/Data/BPS_GameSettings` _gamesettings)))
  (`self.SwitchGameStates` "NewEnumerator0"))

(event `self.K2_PostLogin`
  (params (NewPlayer :type "PlayerController Object Reference"))
  (bind _aspc_gameplay (cast `/Game/S020301L/Blueprints/PlayerControllers/PC_Gameplay` NewPlayer))
  (bind _returnvalue (`KismetArrayLibrary.Array_Add` (`self.Player Controllers`) _aspc_gameplay))
  (`KismetSystemLibrary.PrintString` (`KismetStringLibrary.Conv_IntToString` _returnvalue)))

(event `self.K2_OnLogout`
  (params (ExitingController :type "Controller Object Reference"))
  (bind _aspc_gameplay (cast `/Game/S020301L/Blueprints/PlayerControllers/PC_Gameplay` ExitingController))
  (`KismetArrayLibrary.Array_RemoveItem` (`self.Player Controllers`) _aspc_gameplay))

(fn `CheckIfEnd`
  (locals (AmountSpectating :type Integer))
  (for _array_element (`self.Player Controllers`)
    (bind _isspectating (`/Game/S020301L/Blueprints/PlayerControllers/PC_Gameplay.GetIsSpectating` _array_element))
    (if _isspectating
      (bind _result (`/Engine/EditorBlueprintResources/StandardMacros.IncrementInt` (`local.AmountSpectating`))
        (:`  `
          (set `local.AmountSpectating` _result)))))
  (if (== (`local.AmountSpectating`) (`KismetArrayLibrary.Array_Length` (`self.Player Controllers`)))
    (`self.SwitchGameStates` "NewEnumerator2")))

(fn `Get Player HUD`
  (params (`Player Controller` :type "/Game/S020301L/Blueprints/PlayerControllers/PC_Gameplay Object Reference (by ref)"))
  (returns (Output :type "Widget Object Reference"))
  (return (`|GetArrayItem` (`self.Player HUD`) (`KismetArrayLibrary.Array_Find` (`self.Player Controllers`) `Player Controller`))))

(fn `In-Game Setup`
  (locals (NewLocalVar :type "/Game/S020301L/Blueprints/BP_LavaManager Object Reference"))
  (for _array_element (`self.Player Controllers`)
    (`self.EnableInput` (`Controller.K2_GetPawn` _array_element) null))
  (bind _returnvalue (`|SpawnActorFromClass` "/Game/S020301L/Blueprints/BP_LavaManager.BP_LavaManager_C" (`self.NewMacro`) "AdjustIfPossibleButAlwaysSpawn" "OverrideRootScale" null null))
  (bind _output_get (set `self.LavaManager` _returnvalue))
  (`/Game/S020301L/Blueprints/BP_LavaManager.Init` _output_get (`self.Player HUD`) self)
  (add `/Game/S020301L/Blueprints/BP_LavaManager.OnLavaFinished` _returnvalue (`|CreateDelegate` :!event `Post-Game Setup`)))

(fn `Post-Game Setup`
  (locals (`Surviving Controllers` :type "Array of /Game/S020301L/Blueprints/PlayerControllers/PC_Gameplay Object Reference") (`Dead Controllers` :type "Array of /Game/S020301L/Blueprints/PlayerControllers/PC_Gameplay Object Reference"))
  (for _array_element (`self.Player Controllers`)
    (bind _isspectating (`/Game/S020301L/Blueprints/PlayerControllers/PC_Gameplay.GetIsSpectating` _array_element))
    (if _isspectating
      (`KismetArrayLibrary.Array_Add` (`local.Dead Controllers`) _array_element)
      (else
        (`KismetArrayLibrary.Array_Add` (`local.Surviving Controllers`) _array_element))))
  (`|ExecutionSequence`
    (:`then_0`
      (for _array_element_2 (`local.Surviving Controllers`)
        (bind _output (`/Game/S020301L/Blueprints/PlayerControllers/PC_Gameplay.GetAttachedWidget` _array_element_2))
        (`Widget.RemoveFromParent` _output)
        (bind _returnvalue (`|CreateWidget` "/Game/S020301L/UI/UI_PostGame.UI_PostGame_C" _array_element_2))
        (`UserWidget.AddToPlayerScreen` _returnvalue 0)
        (for (_array_element_3 _array_index) (`self.Player Controllers`)
          (if (== _array_element_3 _array_element_2)
            (`/Game/S020301L/UI/UI_PostGame.UpdateWinText_FIL` _returnvalue _array_index)))))
    (:`then_1`
      (for _array_element_4 (`local.Dead Controllers`)
        (bind _output_2 (`/Game/S020301L/Blueprints/PlayerControllers/PC_Gameplay.GetAttachedWidget` _array_element_4))
        (`Widget.RemoveFromParent` _output_2)
        (bind _returnvalue_2 (`|CreateWidget` "/Game/S020301L/UI/UI_PostGame.UI_PostGame_C" _array_element_4))
        (`UserWidget.AddToPlayerScreen` _returnvalue_2 0)
        (for (_array_element_5 _array_index_2) (`self.Player Controllers`)
          (if (== _array_element_5 _array_element_4)
            (`/Game/S020301L/UI/UI_PostGame.UpdateLoseText_FIL` _returnvalue_2 _array_index_2)))))
    (:`then_2`
      (`KismetSystemLibrary.K2_SetTimerDelegate` (`|CreateDelegate` :!event `Reset`) 5.0))))

(fn `Pre-Game Setup`
  (bind _player_controllers (`self.Player Controllers`))
  (`self.Spawn Characters`)
  (bind _playerhud_s (`self.SpawnPlayerHUD` _player_controllers))
  (set `self.Player HUD` _playerhud_s)
  (for _array_element _player_controllers
    (`self.DisableInput` (`Controller.K2_GetPawn` _array_element) null)
    (`KismetSystemLibrary.PrintString` "Hello"))
  (for _array_element_2 (`self.Player HUD`)
    (bind _asui_fil_hud (cast `/Game/S020301L/UI/UI_FIL_HUD` _array_element_2 :!pure true))
    (`/Game/S020301L/UI/UI_FIL_HUD.OnStart` _asui_fil_hud)
    (`/Engine/EditorBlueprintResources/StandardMacros.DoOnce` false
      (:`Completed`
        (add `/Game/S020301L/UI/UI_FIL_HUD.CountdownComplete` _asui_fil_hud (`|CreateDelegate` :!event `In-Game Setup`))))))

(fn `Reset`
  (`/Game/S020301L/Blueprints/Data/BPL_Gameplay.Remove Players`)
  (bind _returnvalue (`GameplayStatics.CreatePlayer` 0))
  (message `/Game/S020301L/Blueprints/Interfaces/BPI_Initialisable.Init` _returnvalue)
  (`GameplayStatics.OpenLevel` "MainMenu_Map"))

(fn `SelectPlayerSpawn`
  (returns (SelectedSpawn :type "PlayerStart Object Reference"))
  (locals (SpawnPoints :type "Array of PlayerStart Object Reference"))
  (bind _outactors (`GameplayStatics.GetAllActorsOfClass` "/Script/Engine.PlayerStart"))
  (bind _output_get (set `local.SpawnPoints` _outactors))
  (return (`KismetArrayLibrary.Array_Random` _output_get)))

(fn `Set Up Controllers`
  (params (`Number of Players` :type Integer))
  (`GameplayStatics.RemovePlayer` (`GameplayStatics.GetPlayerController` 0))
  (for _index (range `Number of Players`)
    (bind _returnvalue (`GameplayStatics.CreatePlayer` _index))
    (message `/Game/S020301L/Blueprints/Interfaces/BPI_Initialisable.Init` _returnvalue)))

(fn `Spawn Characters`
  (bind _gameinstance (`self.GameInstance`))
  (`/Engine/EditorBlueprintResources/StandardMacros.IsValid` _gameinstance
    (:`Is Valid`
      (bind _charactersettings (`/Game/S020301L/Blueprints/BP_GameInstance.GetCharacterSettings` _gameinstance))
      (for (_array_element _array_index) (`self.Player Controllers`)
        (for (_array_element_2 _array_index_2) (`.Char1_10_5D2AB4BB472DBF7414B068B6B5FC3CAA` (break `/Game/S020301L/Blueprints/Data/BPS_CharacterSettings` _charactersettings))
          (if (== _array_index_2 _array_index)
            (bind _selectedspawn (`self.SelectPlayerSpawn`))
            (bind _returnvalue (`|SpawnActorFromClass` _array_element_2 (`self.GetTransform` _selectedspawn) "AdjustIfPossibleButAlwaysSpawn" "OverrideRootScale" null null))
            (`Controller.Possess` _array_element _returnvalue)
            (message `/Game/S020301L/Blueprints/Interfaces/BPI_Character.Init` _returnvalue "NewEnumerator0")))))))

(fn `SpawnPlayerHUD`
  (params (PlayerController :type "Array of /Game/S020301L/Blueprints/PlayerControllers/PC_Gameplay Object Reference"))
  (returns (`PlayerHUD's` :type "Array of Widget Object Reference"))
  (locals (PlayerHUDs :type "Array of Widget Object Reference"))
  (for _array_element PlayerController
    (bind _returnvalue (`|CreateWidget` "/Game/S020301L/UI/UI_FIL_HUD.UI_FIL_HUD_C" _array_element))
    (`UserWidget.AddToPlayerScreen` _returnvalue 0)
    (`KismetArrayLibrary.Array_Add` (`local.PlayerHUDs`) _returnvalue))
  (return (`local.PlayerHUDs`)))

(fn `SwitchGameStates`
  (params (GameState :type "/Game/S020301L/Blueprints/Data/E_GameState Enum" :default "NewEnumerator0"))
  (switch `/Game/S020301L/Blueprints/Data/E_GameState` GameState
    (:`NewEnumerator0`
      (`self.Pre-Game Setup`))
    (:`NewEnumerator1`
      (`self.In-Game Setup`))
    (:`NewEnumerator2`
      (`self.Post-Game Setup`))))

(fn `UserConstructionScript`)