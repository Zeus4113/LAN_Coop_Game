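; BP_Pickup is a spinning speed or jump boost pickup that respawns after being collected.
; Construction script reveals the mesh matching PickupType, and a Timeline started on BeginPlay adds yaw rotation.
; Overlap by BP_MaleCharacter passes type, modifier and duration to its PickupActivated, then hides the pickup and disables collision.
; A timer using the same Duration restores visibility and collision; leftover reset events are empty.
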(event `self.Collider.OnComponentBeginOverlap`
  (params (OverlappedComponent :type "PrimitiveComponent Object Reference") (OtherActor :type "Actor Object Reference") (OtherComp :type "PrimitiveComponent Object Reference") (OtherBodyIndex :type Integer) (bFromSweep :type Boolean) (SweepResult :type "HitResult Structure (by ref)"))
  (if (not (`self.IsHidden`))
    (bind _asbp_male_character (cast `/Game/S020301L/Blueprints/Characters/BP_MaleCharacter` OtherActor))
    (`/Game/S020301L/Blueprints/Characters/BP_MaleCharacter.PickupActivated` _asbp_male_character (`self.Modifer`) (`self.Pickup Type`) (`self.Duration`))
    (`self.SetActorHiddenInGame` true)
    (`PrimitiveComponent.SetCollisionEnabled` (`self.Collider`) "NoCollision")
    (set `self.IsHidden` true)
    (`KismetSystemLibrary.K2_SetTimerDelegate` (delegate `ResetPickup`) (`self.Duration`))))

(event `ResetPickup`
  (`self.SetActorHiddenInGame` false)
  (set `self.IsHidden` false)
  (`PrimitiveComponent.SetCollisionEnabled` (`self.Collider`) "QueryAndPhysics"))

(event `self.ReceiveBeginPlay`
  (bind (_direction _newtrack_0) (`Timeline|Timeline`)
    (:`Update`
      (`self.K2_AddActorWorldRotation` (`KismetMathLibrary.MakeRotator` 0.0 0.0 _newtrack_0)))))

(event `ResetPlayerStats`)

(event `PickupReset`)

(fn `UserConstructionScript`
  (bind _jumpmesh (`self.JumpMesh`))
  (bind _speed_mesh (`self.Speed Mesh`))
  (switch `/Game/S020301L/Blueprints/Data/E_PickupTypes` (`self.Pickup Type`)
    (:`NewEnumerator0`
      (`SceneComponent.SetHiddenInGame` _speed_mesh false true)
      (`SceneComponent.SetVisibility` _speed_mesh true true))
    (:`NewEnumerator1`
      (`SceneComponent.SetHiddenInGame` _jumpmesh false true)
      (`SceneComponent.SetVisibility` _jumpmesh true true))))