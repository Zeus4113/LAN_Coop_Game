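; Game manager for a hot potato match that spawns players, creates their HUDs and runs the round countdown.
; Init possesses characters chosen from GameInstance settings by player index, spawned at random team-matched starts.
; At match start it attaches a BP_HotPotato component to the first Team B player's pawn.
; A one-second looping timer updates every HUD, then signals completion and detaches the potato when time runs out.
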(event `Init`
  (params (PlayerControllers :type "Array of /Game/S020301L/Blueprints/PlayerControllers/PC_Gameplay Object Reference"))
  ;[0.3748 1 0.3747] Initialise
  (bind _output_get (set `self.PlayerControllers` PlayerControllers))
  (`self.SpawnCharacters`)
  (bind _playerhud_s (`self.AddPlayerHUD` _output_get))
  (set `self.Player HUD's` _playerhud_s)
  (`self.OnTimerStart`)
  (`self.OnMatchStart`))

(event `OnTimerStart`
  ;[0.7292 0.8979 1] Timer Management
  (bind _output_get (set `self.IsTimerActive` true))
  (`self.TimerUpdate`)
  (`KismetSystemLibrary.K2_SetTimerDelegate` (delegate `TimerUpdate`) 1.0 _output_get))

(event `OnTimerEnd`
  ;[0.7292 0.8979 1] Timer Management
  (set `self.IsTimerActive` false)
  (`/Engine/EditorBlueprintResources/StandardMacros.IsValid` (`self.PotatoComponent`)
    (:`Is Valid`
      (`self.DetachPotato`))))

(event `TimerUpdate`
  (bind _timeremaining (`self.TimeRemaining`))
  ;[0.7292 0.8979 1] Timer Management
  (if (`self.IsTimerActive`)
    (`/Engine/EditorBlueprintResources/StandardMacros.DecrementFloat` _timeremaining
      (:`  `
        (if (< _timeremaining 0.0)
          (`self.TimerComplete`)
          (`self.OnTimerEnd`)
          (else
            (for _array_element (`self.Player HUD's`)
              (bind _asui_hp_hud (cast `/Game/S020301L/UI/UI_HP_HUD` _array_element))
              (`/Game/S020301L/UI/UI_HP_HUD.UpdateTimerText` _asui_hp_hud (`self.TimeRemaining`)))))))))

(event `OnMatchStart`
  (`KismetSystemLibrary.PrintString` "Spawning Hot Potato")
  (for _array_element (`self.PlayerControllers`)
    (bind _team_id (message `/Game/S020301L/Blueprints/Interfaces/BPI_Teams.GetTeam` _array_element))
    (switch `/Game/S020301L/Blueprints/Data/E_Teams` _team_id
      (:`NewEnumerator2`
        (`self.AttachPotato` (`Controller.K2_GetPawn` _array_element))
        (break)))))

(event `AttachPotato`
  (params (TargetCharacter :type "Pawn Object Reference"))
  (bind _returnvalue (`|AddComponentByClass` TargetCharacter "/Game/S020301L/Blueprints/BP_HotPotato.BP_HotPotato_C"))
  (bind _output_get (set `self.PotatoComponent` _returnvalue))
  (`/Game/S020301L/Blueprints/BP_HotPotato.Init` _output_get TargetCharacter))

(event `DetachPotato`
  (`/Game/S020301L/Blueprints/BP_HotPotato.Detatch` (`self.PotatoComponent`)))

(fn `AddPlayerHUD`
  (params (PlayerControllers :type "Array of /Game/S020301L/Blueprints/PlayerControllers/PC_Gameplay Object Reference"))
  (returns (`PlayerHUD's` :type "Array of /Game/S020301L/UI/UI_HP_HUD Object Reference"))
  (locals (PlayerHUDs :type "Array of /Game/S020301L/UI/UI_HP_HUD Object Reference"))
  (for _array_element PlayerControllers
    (bind _returnvalue (`|CreateWidget` "/Game/S020301L/UI/UI_HP_HUD.UI_HP_HUD_C" _array_element))
    (`UserWidget.AddToPlayerScreen` _returnvalue 0)
    (`KismetArrayLibrary.Array_Add` (`local.PlayerHUDs`) _returnvalue))
  (return (`local.PlayerHUDs`)))

(fn `GetPlayerHUD`
  (params (PlayerController :type "/Game/S020301L/Blueprints/PlayerControllers/PC_Gameplay Object Reference"))
  (returns (Output :type "Widget Object Reference"))
  (return (`|GetArrayItem` (`self.Player HUD's`) (`KismetArrayLibrary.Array_Find` (`self.PlayerControllers`) PlayerController))))

(fn `GetPlayerHUDArray`)

(fn `GetPotato`
  (returns (PotatoComponent :type "/Game/S020301L/Blueprints/BP_HotPotato Object Reference"))
  (return (`self.PotatoComponent`)))

(fn `SelectPlayerSpawn`
  (params (`Team ID` :type "/Game/S020301L/Blueprints/Data/E_Teams Enum" :default "NewEnumerator0"))
  (returns (ChosenSpawnPoint :type "Actor Object Reference"))
  (locals (SpawnPoints :type "Array of /Game/S020301L/Blueprints/BP_TeamPlayerStart Object Reference"))
  (bind _outactors (`GameplayStatics.GetAllActorsOfClass` "/Game/S020301L/Blueprints/BP_TeamPlayerStart.BP_TeamPlayerStart_C"))
  (for _array_element _outactors
    (bind _team_id (message `/Game/S020301L/Blueprints/Interfaces/BPI_Teams.GetTeam` _array_element))
    (if (`|EnumEquality` _team_id `Team ID`)
      (`KismetArrayLibrary.Array_Add` (`local.SpawnPoints`) _array_element)))
  (if (!= (`KismetArrayLibrary.Array_Length` (`local.SpawnPoints`)) 0)
    (return (`KismetArrayLibrary.Array_Random` (`local.SpawnPoints`)))
    (else
      (bind _returnvalue (`GameplayStatics.GetActorOfClass` "/Game/S020301L/Blueprints/BP_TeamPlayerStart.BP_TeamPlayerStart_C"))
      (return _returnvalue))))

(fn `SetPlayerHUDArray`
  (params (NewWidgetArray :type "Array of Widget Object Reference"))
  (set `self.Player HUD's` NewWidgetArray))

(fn `SetPotato`
  (params (NewPotato :type "/Game/S020301L/Blueprints/BP_HotPotato Object Reference"))
  (set `self.PotatoComponent` NewPotato))

(fn `SpawnCharacters`
  (locals (CharSettings :type "/Game/S020301L/Blueprints/Data/BPS_CharacterSettings Structure"))
  (bind _asbp_game_instance (cast `/Game/S020301L/Blueprints/BP_GameInstance` (`GameplayStatics.GetGameInstance`)))
  (bind _charactersettings (`/Game/S020301L/Blueprints/BP_GameInstance.GetCharacterSettings` _asbp_game_instance))
  (for (_array_element _array_index) (`self.PlayerControllers`)
    (for (_array_element_2 _array_index_2) (`.Char1_10_5D2AB4BB472DBF7414B068B6B5FC3CAA` (break `/Game/S020301L/Blueprints/Data/BPS_CharacterSettings` _charactersettings))
      (if (== _array_index_2 _array_index)
        (bind _team_id (`/Game/S020301L/Blueprints/Interfaces/BPI_Teams.GetTeam` _array_element))
        (bind _returnvalue (`|SpawnActorFromClass` _array_element_2 (`self.GetTransform` (`self.SelectPlayerSpawn` _team_id)) "AdjustIfPossibleButAlwaysSpawn" "OverrideRootScale" null null))
        (`Controller.Possess` _array_element _returnvalue)
        (message `/Game/S020301L/Blueprints/Interfaces/BPI_Character.Init` _returnvalue _team_id)))))

(fn `UserConstructionScript`)