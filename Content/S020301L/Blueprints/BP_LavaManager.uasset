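; BP_LavaManager raises the level's lava floor over time and reports its progress to player HUDs.
; Init stores the HUD array, finds the BP_LavaFloor actor and, if it exists, starts the rise.
; The LavaRaise timeline lerps the floor from its start location by TravelDistance.
; Each update converts the distance covered into a rounded percentage and pushes it to every UI_FIL_HUD.
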(event `Init`
  (params (PlayerHUD :type "Array of Widget Object Reference"))
  (set `self.Player HUD` PlayerHUD)
  (bind _returnvalue (`GameplayStatics.GetActorOfClass` "/Game/S020301L/Blueprints/BP_LavaFloor.BP_LavaFloor_C"))
  (bind _output_get (set `self.LavaFloor` _returnvalue))
  (`/Engine/EditorBlueprintResources/StandardMacros.IsValid` _output_get
    (:`Is Valid`
      (`self.StartLavaRaise`))))

(event `StartLavaRaise`
  (bind _startposition (`self.StartPosition`))
  (bind _output_get (set `self.StartPosition` (`self.K2_GetActorLocation` (`self.LavaFloor`))))
  (set `self.TargetPosition` (+ _output_get (`self.TravelDistance`)))
  (set `self.TotalDistance` (`KismetMathLibrary.VSize` (- (`self.StartPosition`) (`self.TargetPosition`))))
  (bind (_direction _newtrack_0) (`Timeline|LavaRaise`)
    (:`Update`
      (bind _returnvalue (`KismetMathLibrary.VLerp` _startposition (`self.TargetPosition`) _newtrack_0))
      (`self.K2_SetActorLocation` (`self.LavaFloor`) _returnvalue false false)
      (`self.UpdateHUD` (`KismetMathLibrary.VSize` (- _startposition _returnvalue))))
    (:`Finished`
      (`KismetSystemLibrary.PrintString` "Complete"))))

(event `UpdateHUD`
  (params (CurrentDistance :type "Float (double-precision)"))
  (for _array_element (`self.Player HUD`)
    (`/Game/S020301L/UI/UI_FIL_HUD.UpdateLavaPercent` (cast `/Game/S020301L/UI/UI_FIL_HUD` _array_element :!pure true) (`KismetMathLibrary.Conv_IntToDouble` (`KismetMathLibrary.Round` (* (/ CurrentDistance (`self.TotalDistance`)) 100.0))))))

(fn `UserConstructionScript`)