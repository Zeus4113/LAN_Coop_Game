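; BP_HPGameManager is a game manager Blueprint that runs a countdown timer.
; StartTimer sets a running flag, ticks once immediately and sets a looping one-second timer on UpdateTimer.
; Each tick decrements CurrentTime and calls TimerUpdate with it, or calls TimerComplete and stops once it drops below zero.
; StopTimer only lowers the flag, so the looping timer keeps firing without effect.
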(event `Stop Timer`
  ;[0.528 0.8267 1] Timer Functionality
  (set `self.IsTimerRunning` false))

(event `Start Timer`
  ;[0.528 0.8267 1] Timer Functionality
  (set `self.IsTimerRunning` true)
  (`self.Update Timer`)
  (`KismetSystemLibrary.K2_SetTimerDelegate` (delegate `Update Timer`) 1.0 true)
  (`KismetSystemLibrary.PrintString` "Timer Starting"))

(event `Update Timer`
  (bind _currenttime (`self.CurrentTime`))
  ;[0.528 0.8267 1] Timer Functionality
  (if (`self.IsTimerRunning`)
    (`/Engine/EditorBlueprintResources/StandardMacros.DecrementInt` _currenttime
      (:`  `
        (if (< _currenttime 0)
          (`self.TimerComplete`)
          (`self.Stop Timer`)
          (else
            (`self.TimerUpdate` (`self.CurrentTime`))))))))

(fn `UserConstructionScript`)