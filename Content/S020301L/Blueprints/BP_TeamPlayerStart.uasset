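; BP_TeamPlayerStart is a player start marker that carries a team ID: NoTeam, TeamA or TeamB.
; SetTeam assigns the ID and GetTeam returns it for other code to read.
; The construction script shows the team name on a text render component, with its color selected by team.
; SetTeam changes only the variable and does not refresh the label itself.
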(event `/Game/S020301L/Blueprints/Interfaces/BPI_Teams.SetTeam`
  (params (`Team ID` :type "/Game/S020301L/Blueprints/Data/E_Teams Enum" :default "NewEnumerator0"))
  (set `self.Team ID` `Team ID`))

(fn `GetTeam`
  (returns (`Team ID` :type "/Game/S020301L/Blueprints/Data/E_Teams Enum"))
  (return (`self.Team ID`)))

(fn `UserConstructionScript`
  (bind _textrender (`self.TextRender`))
  (`TextRenderComponent.K2_SetText` _textrender (`KismetTextLibrary.Conv_StringToText` (`|GetEnumeratorNameAsString` (`self.Team ID`))))
  (`TextRenderComponent.SetTextRenderColor` _textrender (select `/Game/S020301L/Blueprints/Data/E_Teams` (`self.Team ID`) :`NewEnumerator0` (make `Color` :`G` 255) :`NewEnumerator1` (make `Color` :`B` 255) :`NewEnumerator2` (make `Color` :`R` 255))))