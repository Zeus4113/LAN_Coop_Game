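; Gameplay player controller for a potato-timer mode, holding each player's team, health and accumulated time as potato.
; Health loads from PlayerStats; damage adds health for a matching team and subtracts otherwise, checked against both instigator and damage causer, so each hit applies twice.
; Added potato time updates the player's HUD, fetched through GM_HP's game manager.
; It also toggles pawn input and exits to the main menu, removing players.
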(event `InputAction|ExitLevel`
  (params (Key :type "Key Structure"))
  (:`Pressed`
    (`/Game/S020301L/Blueprints/Data/BPL_Gameplay.Remove Players`)
    (`GameplayStatics.OpenLevel` "MainMenu_Map")))

(event `/Game/S020301L/Blueprints/Interfaces/BPI_Initialisable.Init`
  (bind (_currenthealth _maxhealth) (break `/Game/S020301L/Blueprints/Data/BPS_PlayerStats` (`self.PlayerStats`)))
  (set `self.Current Health` _currenthealth)
  (set `self.Max Health` _maxhealth))

(event `/Game/S020301L/Blueprints/Interfaces/BPI_Teams.SetTeam`
  (params (`Team ID` :type "/Game/S020301L/Blueprints/Data/E_Teams Enum" :default "NewEnumerator0"))
  (set `self.Team ID` `Team ID`))

(event `self.ReceiveAnyDamage`
  (params (Damage :type "Float (single-precision)") (DamageType :type "DamageType Object Reference") (InstigatedBy :type "Controller Object Reference") (DamageCauser :type "Actor Object Reference"))
  (bind _team_id (`self.Team ID`))
  (`|ExecutionSequence`
    (:`then_0`
      (bind _team_id_2 (message `/Game/S020301L/Blueprints/Interfaces/BPI_Teams.GetTeam` InstigatedBy))
      (if (`|EnumEquality` _team_id_2 _team_id)
        (bind _output_get (set `self.Current Health` (+ (`self.Current Health`) Damage) :!label _label))
        (else
          (set `self.Current Health` (- (`self.Current Health`) Damage) :!label _label_2))))
    (:`then_1`
      (bind _team_id_3 (message `/Game/S020301L/Blueprints/Interfaces/BPI_Teams.GetTeam` DamageCauser))
      (if (`|EnumEquality` _team_id _team_id_3)
        (goto _label)
        (else
          (goto _label_2)))))
  (`KismetSystemLibrary.PrintString` (`KismetStringLibrary.Conv_DoubleToString` _output_get)))

(event `SetTotalTime`
  (params (`New Time` :type "Float (double-precision)"))
  (bind _output_get (set `self.TimeAsPotato` (+ `New Time` (`self.TimeAsPotato`))))
  (bind _output (`self.GetAttachedWidget`))
  (`/Game/S020301L/UI/UI_HP_HUD.UpdatePotatoTimer` _output _output_get))

(fn `CanInput`
  (params (`CanInput?` :type Boolean))
  (bind _returnvalue (`self.K2_GetPawn` self))
  (if `CanInput?`
    (`self.EnableInput` _returnvalue self)
    (else
      (`self.DisableInput` _returnvalue self))))

(fn `GetAttachedWidget`
  (returns (Output :type "/Game/S020301L/UI/UI_HP_HUD Object Reference"))
  (bind _asgm_hp (cast `/Game/S020301L/Blueprints/Gamemodes/GM_HP` (`GameplayStatics.GetGameMode`)))
  (bind _gamemanager (`/Game/S020301L/Blueprints/Gamemodes/GM_HP.GetGameManager` _asgm_hp))
  (bind _output (`/Game/S020301L/Blueprints/BP_GameManager.GetPlayerHUD` _gamemanager self))
  (return _output))

(fn `GetTeam`
  (returns (`Team ID` :type "/Game/S020301L/Blueprints/Data/E_Teams Enum"))
  (return (`self.Team ID`)))

(fn `GetTotalTime`
  (returns (TimeAsPotato :type "Float (double-precision)"))
  (return (`self.TimeAsPotato`)))

(fn `UserConstructionScript`)